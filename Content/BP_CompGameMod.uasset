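; BP_CompGameMod, apparently a game mode by its name, starts playback of a green screen video when play begins.
; On BeginPlay it prints the current level name, opens GreenScreen.mp4 from the project Content directory as a file URL on the VideoInput media player, and calls Play immediately.
; Tick and the construction script are empty, and leftover path-printing nodes are disconnected.
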(event `self.ReceiveBeginPlay`
  (bind _returnvalue (`GameplayStatics.GetCurrentLevelName` true))
  (`KismetSystemLibrary.PrintString` _returnvalue)
  (`MediaPlayer.OpenUrl` (`self.VideoInput`) (`KismetStringLibrary.Concat_StrStr` "file://" (`KismetSystemLibrary.GetProjectContentDirectory`) "GreenScreen.mp4"))
  (bind _returnvalue_2 (`MediaPlayer.Play` (`self.VideoInput`))))

(fn `UserConstructionScript`)