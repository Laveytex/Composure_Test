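; Composure controller that builds a green-screen compositing hierarchy in code and refreshes the element list and viewport every tick.
; CreateComposElements, not called within the graph, creates a Main plate with Media and CG child plates.
; Media chroma-keys and erodes a test texture, CG reads a camera render target, and Main targets a CineCamera, adding an overlay material and player-viewport output.
; Many disconnected experimental chains remain.
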(event `self.ReceiveBeginPlay`)

(event `self.ReceiveTick`
  (params (DeltaSeconds :type "Float (single-precision)"))
  (`ComposureBlueprintLibrary.RefreshComposureElementList`)
  (`ComposureBlueprintLibrary.RequestRedrawComposureViewport`))

(event `CreateComposElements`
  (`|ExecutionSequence`
    (:`then_0`
      (bind _returnvalue (`GameplayStatics.GetActorOfClass` "/Script/Engine.LevelScriptActor"))
      (bind _compelement (`self.Create Comp Element` "Main_Plate" "/Script/Composure.CompositingElement" _returnvalue))
      (bind _returnvalue_2 (`|SpawnActorFromClass` (`GameplayStatics.GetObjectClass` _compelement) (`self.Spawn Transform`) "Undefined" "OverrideRootScale" null null))
      (bind _output_get (set `self.MainComposureElement` _returnvalue_2))
      (bind _compelement_2 (`self.Create Comp Element` "Media_Plate" "/Script/Composure.CompositingElement" _output_get))
      (bind _returnvalue_3 (`|SpawnActorFromClass` (`GameplayStatics.GetObjectClass` _compelement_2) (`self.Spawn Transform`) "Undefined" "OverrideRootScale" null null))
      (bind _output_get_2 (set `self.MediaComposureElement` _returnvalue_3))
      (`ComposureBlueprintLibrary.AttachComposureElement` "Main_Plate" "Media_Plate")
      (`self.K2_AttachToActor` _output_get_2 (`self.MainComposureElement`) "None" "KeepRelative" "KeepRelative" "KeepRelative" false)
      (bind _compelement_3 (`self.Create Comp Element` "CG_Plate" "/Script/Composure.CompositingElement" _returnvalue))
      (bind _returnvalue_4 (`|SpawnActorFromClass` (`GameplayStatics.GetObjectClass` _compelement_3) (`self.Spawn Transform`) "Undefined" "OverrideRootScale" null null))
      (bind _output_get_3 (set `self.CGComposureElement` _returnvalue_4))
      (`ComposureBlueprintLibrary.AttachComposureElement` "Main_Plate" "CG_Plate")
      (`self.K2_AttachToActor` _output_get_3 (`self.MainComposureElement`) "None" "KeepRelative" "KeepRelative" "KeepRelative" false)
      (`self.MainComposInstal` "None")
      (`self.MediaComposInstal` false)
      (`self.CGComposInstal`))))

(event `MainComposInstal`
  (params (ElementName :type Name))
  (`|ExecutionSequence`
    (:`then_0`
      (bind _returnvalue (`GameplayStatics.GetActorOfClass` "/Script/CinematicCamera.CineCameraActor"))
      (bind _ascine_camera_actor (cast `CineCameraActor` _returnvalue))
      (bind _output_get (set `self.As Cine Camera Actor` _ascine_camera_actor))
      (`CompositingElement.SetTargetCamera` (`self.MainComposureElement`) _output_get))
    (:`then_1`
      (bind _returnvalue_2 (`CompositingElement.CreateNewTransformPass` (`self.MainComposureElement`) "OverTransform" "/Script/Composure.CompositingElementMaterialPass"))
      (`CompositingElementMaterialPass.SetMaterialInterface` _returnvalue_2 "/Game/M_OverLeyer.M_OverLeyer")
      (bind _returnvalue_3 (`CompositingElementMaterialPass.SetParameterMapping` _returnvalue_2 "Media" "CompositingElement1"))
      (`KismetSystemLibrary.PrintString` (`KismetStringLibrary.Conv_BoolToString` _returnvalue_3))
      (bind _returnvalue_4 (`CompositingElementMaterialPass.SetParameterMapping` _returnvalue_2 "CG" "BP_CgCaptureCompElement0"))
      (`KismetSystemLibrary.PrintString` (`KismetStringLibrary.Conv_BoolToString` _returnvalue_4)))
    (:`then_2`
      (`CompositingElement.CreateNewOutputPass` (`self.MainComposureElement`) "MainOut" "/Script/Composure.PlayerViewportCompositingOutput"))))

(event `MediaComposInstal`
  (params (IsHave :type Boolean) (PassName :type Name))
  (bind _mediacomposureelement (`self.MediaComposureElement`))
  (`|ExecutionSequence`
    (:`then_0`
      (bind _returnvalue (`CompositingElement.CreateNewTransformPass` (`self.MediaComposureElement`) "Chromakey" "/Script/Composure_Test.ComposureKeyColorMaterialTransform"))
      (`ComposureKeyColorMaterialTransform.SetMaterial` _returnvalue "/Composure/Materials/ChromaKeying/M_SinglePassChromaKeyer.M_SinglePassChromaKeyer")
      (`ComposureKeyColorMaterialTransform.SetKey` _returnvalue (struct :`G` 1.0 :`B` 0.037633 :`A` 1.0))
      (`ComposureKeyColorMaterialTransform.SetKey` _returnvalue (struct :`G` 1.0 :`B` 0.037633 :`A` 1.0))
      (`ComposureKeyColorMaterialTransform.SetMaterialParams` _returnvalue 0.455038 4.0 1.0 1.0 0.0 1.0 1.0 0.0 0.0 0.5 0.0 100.0))
    (:`then_1`
      (bind _returnvalue_2 (`CompositingElement.CreateNewTransformPass` (`self.MediaComposureElement`) "Erod" "/Script/Composure_Test.ComposureScalarMaterialTransform"))
      (`ComposureScalarMaterialTransform.SetMaterial` _returnvalue_2 "/Composure/Materials/ChromaKeying/ErodeAlpha.ErodeAlpha"))
    (:`then_3`
      (bind _returnvalue_3 (`CompositingElement.CreateNewInputPass` _mediacomposureelement "MediaTransform" "/Composure/Blueprints/CompositingPasses/BP_TextureCompInput.BP_TextureCompInput_C"))
      (bind _output_get (set `/Composure/Blueprints/CompositingPasses/BP_TextureCompInput.TextureInput` "/Game/TestCompMedia_InnerAssets/T_TestCompMedia_BC.T_TestCompMedia_BC" _returnvalue_3))
      (`ComposureCompositingTargetComponent.SetDisplayTexture` (`CompositingElement.CompositingTarget` _mediacomposureelement) _output_get))))

(event `CGComposInstal`
  (bind _returnvalue (`CompositingElement.CreateNewInputPass` (`self.CGComposureElement`) "CamInput" "/Composure/Blueprints/CompositingPasses/BP_TextureCompInput.BP_TextureCompInput_C"))
  (set `/Composure/Blueprints/CompositingPasses/BP_TextureCompInput.TextureInput` "/Game/RT_CamView.RT_CamView" _returnvalue))

(fn `Create Comp Element`
  (params (CompElementName :type Name) (CompClassType :type "CompositingElement Class Reference") (LevelContext :type "Actor Object Reference"))
  (returns (CompElement :type "CompositingElement Object Reference"))
  (locals (`IsElement?` :type Boolean) (CompElement2 :type "CompositingElement Object Reference"))
  (`/Engine/EditorBlueprintResources/StandardMacros.IsValid` (`ComposureBlueprintLibrary.GetComposureElement` CompElementName)
    (:`Is Valid`
      (`ComposureBlueprintLibrary.DeleteComposureElementAndChildren` CompElementName))
    (:`Is Not Valid`
      _))
  (bind _returnvalue (`ComposureBlueprintLibrary.CreateComposureElement` CompElementName CompClassType null))
  (set `local.CompElement2` _returnvalue)
  (return (`local.CompElement2`)))

(fn `UserConstructionScript`)